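; Countdown timer actor for a timed objective: overlapping EndTarget before time runs out succeeds and removes the timer and its widget.
; Each Tick decrements TimeRemaining and writes it to a CountdownTime_UI_BP widget created on BeginPlay.
; On expiry, IsRecoverable resets time and applies the stored player transform, otherwise the actor and widget are removed.
; That "starting" transform is re-captured every tick, so it holds the player's current position.
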(event OnComponentBeginOverlap(EndTarget)
  (params (OverlappedComponent :type Primitive%20Component%20Object%20Reference) (OtherActor :type Actor%20Object%20Reference) (OtherComp :type Primitive%20Component%20Object%20Reference) (OtherBodyIndex :type Integer) (bFromSweep :type Boolean) (SweepResult :type Hit%20Result%20Structure%20%28by%20ref%29))
  ;[1 1 1] If player reaches the target before time runs out - success
  (Development|PrintString "End countdown - success")
  (Development|PrintString "Check - if carrying something, destroy it")
  (Widget|RemovefromParent (stale EventBeginPlay _returnvalue))
  (Actor|DestroyActor))

(event Custom|Timer
  ;[1 1 1] Timer Countdown
  ;;[1 1 1] Set 3rd Person location
  (bind _returnvalue (Actor|GetActorOfClass "/Game/ThirdPerson/Blueprints/BP_ThirdPersonCharacter.BP_ThirdPersonCharacter_C"))
  (Variables|Default|SetstartingPositionOf3rdPersonCharacter (Transformation|GetActorTransform _returnvalue))
  (Variables|Default|SetTime_Remaining (- (Variables|Default|GetTime_Remaining) (Utilities|Time|GetWorldDeltaSeconds)))
  ;;[1 1 1] Fail State - if Time Remaining <= 0
  (if (not (>= (Variables|Default|GetTime_Remaining) 0.0))
    (Development|PrintString "Time expired, mission has failed")
    (if (Variables|Default|Getis_Recoverable)
      ;;[1 1 1] If it is repeatable (Mission) - restore time, restart player position
      (bind _returnvalue_2 (Actor|GetActorOfClass "/Game/ThirdPerson/Blueprints/BP_ThirdPersonCharacter.BP_ThirdPersonCharacter_C"))
      (Transformation|SetWorldTransform (Variables|/Script/Engine.Actor|GetRootComponent _returnvalue_2) (Variables|Default|GetstartingPositionOf3rdPersonCharacter) false false)
      (Variables|Default|SetTime_Remaining (Variables|Default|GetStarting_Time))
      (else
        ;;[1 1 1] If not repeatable (World Event) - destroy the opportunity
        (Widget|RemovefromParent (stale EventBeginPlay _returnvalue))
        (Actor|DestroyActor)))))

(event EventBeginPlay
  (bind _returnvalue (UserInterface|CreateWidget "/Game/Blueprints/CountdownTime_UI_BP.CountdownTime_UI_BP_C"))
  (Variables|Default|SetText%20Block%20Changing%20Time (Variables|/Game/Blueprints/CountdownTime_UI_BP.CountdownTime_UI_BP_C|GetTextBlock_ChangingTime _returnvalue))
  (UserInterface|Viewport|AddtoViewport _returnvalue 0))

(event EventTick
  (params (DeltaSeconds :type Float%20%28single-precision%29))
  ;[1 1 1] Update the timer every frame
  (CallFunction|Timer)
  (Rendering|Components|TextRender|SetText (Variables|Default|GetText%20Block%20Changing%20Time) (Utilities|Text|ToText(Float) (Variables|Default|GetTime_Remaining) "HalfToEven")))

(fn ConstructionScript)