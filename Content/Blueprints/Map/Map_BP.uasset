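; Actor component that toggles a pausing map screen backed by a scene capture camera on its owner.
; BeginPlay caches the owner's SceneCaptureComponent2D as the map camera.
; ToggleMap either removes an existing Map_Widget and restores game input, or pauses, creates the widget with the camera and switches to UI-only input.
; Opening the map also resets the camera's position, rotation and ortho width.
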(event EventBeginPlay
  (Variables|Default|SetMapCamera (Actor|GetComponentbyClass (Components|GetOwner) "/Script/Engine.SceneCaptureComponent2D")))

(fn ToggleMap
  (bind _returnvalue (Game|GetPlayerController 0))
  (bind _returnvalue_2 (Game|GetPlayerController 0))
  (bind _foundwidgets (Widget|GetAllWidgetsOfClass "/Game/Blueprints/Map/Map_Widget.Map_Widget_C" true))
  (if (Utilities|IsValid (Utilities|Array|Get(acopy) _foundwidgets))
    (Widget|RemovefromParent (Utilities|Array|Get(acopy) _foundwidgets))
    (Input|SetInputModeGameOnly _returnvalue_2 false)
    (Variables|/Script/Engine.PlayerController|SetbShowMouseCursor _returnvalue_2 false)
    (Game|SetGamePaused false)
    (else
      (Game|SetGamePaused true)
      (bind _returnvalue_3 (UserInterface|CreateWidget "/Game/Blueprints/Map/Map_Widget.Map_Widget_C"))
      (Variables|/Game/Blueprints/Map/Map_Widget.Map_Widget_C|SetMapCamera _returnvalue_3 (Variables|Default|GetMapCamera))
      (UserInterface|Viewport|AddtoViewport _returnvalue_3 0)
      (Input|SetInputModeUIOnly _returnvalue _returnvalue_3 "LockAlways" false)
      (Variables|/Script/Engine.PlayerController|SetbShowMouseCursor _returnvalue true)
      (Transformation|SetRelativeLocation (Variables|Default|GetMapCamera) "0, 0, 0" false true)
      (Transformation|SetWorldRotation (Variables|Default|GetMapCamera) "270.000000,0.000000,0.000000" false false)
      (Variables|/Script/Engine.SceneCaptureComponent2D|SetOrthoWidth (Variables|Default|GetMapCamera) 5e+03))))