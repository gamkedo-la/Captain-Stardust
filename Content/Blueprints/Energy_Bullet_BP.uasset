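; Energy bullet projectile that bursts into shrapnel on impact and self-destructs after a short lifetime.
; Sphere overlaps branch on actor tags: shields destroy it, buildings spawn scale-based debris and destroy it, while enemies and houses spawn type-specific shrapnel without destroying it.
; While the player is targeting, Tick adds a scene component to the targeted actor every frame and makes it the gravity-free homing target.
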(event OnComponentBeginOverlap(Sphere1)
  (params (OverlappedComponent :type Primitive%20Component%20Object%20Reference) (OtherActor :type Actor%20Object%20Reference) (OtherComp :type Primitive%20Component%20Object%20Reference) (OtherBodyIndex :type Integer) (bFromSweep :type Boolean) (SweepResult :type Hit%20Result%20Structure%20%28by%20ref%29))
  (if (Actor|ActorHasTag OtherActor "QuasarShield")
    (Actor|DestroyActor)
    (else
      ;[1 1 1] Hit Building Collision
      (if (Actor|ActorHasTag OtherActor "Building")
        (if (<= (.x (Transformation|GetActorScale3D)) 0.2)
          (for _index (range 0 (Math|Random|RandomIntegerinRange 1 5))
            (Game|SpawnActorfromClass "/Game/Blueprints/Shrapnel/Shrapnel1.Shrapnel1_C" (Transformation|GetActorTransform) "Undefined" "MultiplyWithRoot" 0 0))
          (elif (< (.x (Transformation|GetActorScale3D)) 0.5)
            (for _index_2 (range 0 (Math|Random|RandomIntegerinRange 5 15))
              (Game|SpawnActorfromClass "/Game/Blueprints/Shrapnel/Shrapnel1.Shrapnel1_C" (Transformation|GetActorTransform) "Undefined" "MultiplyWithRoot" 0 0))
            (else
              (for _index_3 (range 0 (Math|Random|RandomIntegerinRange 15 30))
                (Game|SpawnActorfromClass "/Game/Blueprints/Shrapnel/Shrapnel1.Shrapnel1_C" (Transformation|GetActorTransform) "Undefined" "MultiplyWithRoot" 0 0)))))
        (Actor|DestroyActor)
        (elif (Actor|ActorHasTag OtherActor "Enemy")
          ;[1 1 1] if hit enemy, create shrapnel
          (if (Actor|ActorHasTag OtherActor "Robber")
            ;[1 1 1] Mugger Shrapnel
            (for _index_4 (range 0 (Math|Random|RandomIntegerinRange 2 4))
              (Game|SpawnActorfromClass "/Game/Blueprints/Shrapnel/Shrapnel7.Shrapnel7_C" (Transformation|GetActorTransform) "Undefined" "MultiplyWithRoot" 0 0))
            (else
              (for _index_5 (range 0 (Math|Random|RandomIntegerinRange 7 10))
                (Game|SpawnActorfromClass "/Game/Blueprints/Shrapnel/Shrapnel2.Shrapnel2_C" (Transformation|GetActorTransform) "Undefined" "MultiplyWithRoot" 0 0))))
          (else
            ;[1 1 1] House collision
            (if (Actor|ActorHasTag OtherActor "House")
              (bind _ashouse_bp (Utilities|Casting|CastToHouse_BP OtherActor))
              (for _index_6 (range 0 (Math|Random|RandomIntegerinRange 7 15))
                (Game|SpawnActorfromClass (Variables|/Game/Blueprints/House_BP.House_BP_C|GetShrapnel1 _ashouse_bp) (Transformation|GetActorTransform) "Undefined" "MultiplyWithRoot" 0 0)))))))))

(event EventBeginPlay
  (Utilities|FlowControl|Delay 4.0)
  (Actor|DestroyActor))

(event EventTick
  (params (DeltaSeconds :type Float%20%28single-precision%29))
  (bind _projectilemovement (Variables|Default|GetProjectileMovement))
  ;[0.625 0.625 0.625] Targeting with homing energy strike if player is targeting them
  (bind _asbp_third_person_character (Utilities|Casting|CastToBP_ThirdPersonCharacter (Game|Player|GetPlayerPawn 0)))
  (if (Variables|/Game/ThirdPerson/Blueprints/BP_ThirdPersonCharacter.BP_ThirdPersonCharacter_C|GetisTargeting _asbp_third_person_character)
    (bind _returnvalue (AddComponent|AddSceneComponent (Variables|/Game/ThirdPerson/Blueprints/BP_ThirdPersonCharacter.BP_ThirdPersonCharacter_C|GetTargeted%20Actor _asbp_third_person_character) false))
    (Variables|/Script/Engine.ProjectileMovementComponent|SetHomingTargetComponent _projectilemovement _returnvalue)
    (Variables|/Script/Engine.ProjectileMovementComponent|SetbIsHomingProjectile _projectilemovement true)
    (Variables|/Script/Engine.ProjectileMovementComponent|SetHomingAccelerationMagnitude _projectilemovement 1e+05)
    (Variables|/Script/Engine.ProjectileMovementComponent|SetProjectileGravityScale _projectilemovement 0.0)))

(fn ConstructionScript)