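; AI controller for city pedestrians that switches on the possessed CityPerson_BP's State every Tick.
; The first three states call MoveForward, which ground-traces then issues MoveTo or lowers the pawn, though Tick passes it zero DeltaTime.
; Search faces the nearest sidewalk and aligns on arrival, flee faces away from the nearest mugger, and ragdoll resets after landing.
; The normal-state sidewalk check is never run.
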(event EventBeginPlay)

(event EventTick
  (params (DeltaSeconds :type Float%20%28single-precision%29))
  (bind _ascity_person_bp (Utilities|Casting|CastToCityPerson_BP (Pawn|GetControlledPawn)))
  (switch int (Variables|/Game/Blueprints/CityPerson_BP.CityPerson_BP_C|GetState _ascity_person_bp)
    (:0
      (CallFunction|MoveForward 0.0))
    (:1
      (CallFunction|MoveForward 0.0)
      (|SearchState_2))
    (:2
      (CallFunction|MoveForward 0.0)
      (|FleeState_2))
    (:3
      (|RagdollState_2))))

(fn ConstructionScript)

(fn MoveForward
  (params (DeltaTime :type Float%20%28double-precision%29))
  (bind _returnvalue (Pawn|GetControlledPawn))
  (bind _returnvalue_2 (Pawn|GetControlledPawn))
  (bind _returnvalue_3 (Pawn|GetControlledPawn))
  (bind _rootcomponent (Variables|/Script/Engine.Actor|GetRootComponent _returnvalue))
  (bind _rootcomponent_2 (Variables|/Script/Engine.Actor|GetRootComponent _returnvalue_2))
  (bind _rootcomponent_3 (Variables|/Script/Engine.Actor|GetRootComponent _returnvalue_3))
  (bind _returnvalue_4 (Transformation|GetWorldLocation _rootcomponent_2))
  (bind (_outhit _returnvalue_5) (Collision|LineTraceByChannel _returnvalue_4 (+ _returnvalue_4 (Math|Vector|MakeVector 0.0 0.0 -1e+02)) "TraceTypeQuery1" false (Utilities|Array|MakeArray (Game|GetPlayerCharacter 0)) "None"))
  (if _returnvalue_5
    (AI|Navigation|MovetoLocation (AI|GetAIController self) (Math|Vector|SelectVector (+ (* (Variables|Default|GetSpeed) DeltaTime (Math|Vector|GetForwardVector _rootcomponent_3)) (Transformation|GetWorldLocation _rootcomponent_3) (Math|Vector|SelectVector (Math|Vector|VectorUp) (Math|Vector|VectorZero) (and (<= (.Distance (Collision|BreakHitResult _outhit)) 8e+01) (Utilities|Enum|Equal(Enum) (Variables|/Script/Engine.SceneComponent|GetMobility (.HitComponent (Collision|BreakHitResult _outhit))) "Static")))) "0, 0, 0" _returnvalue_5) 0.0 true true false true 0)
    (else
      (Transformation|SetWorldLocation _rootcomponent (+ (Math|Vector|VectorDown) (Transformation|GetWorldLocation _rootcomponent)) false false))))