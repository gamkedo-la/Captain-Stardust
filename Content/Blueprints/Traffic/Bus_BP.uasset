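; Traffic bus that drives along a spline, optionally looping, with a random material picked at BeginPlay.
; A front sensor halts it for players, enemies, vehicles and people, and resumes it on end overlap.
; Tagged attacks and non-Robber enemies drain health, spawning shrapnel, then smoke and a stall, then an explosion and delayed reset to the start.
; PickUp stops movement, and Release leaves it smoking and immobile at one health.
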(event OnComponentBeginOverlap(BusMesh)
  (params (OverlappedComponent :type Primitive%20Component%20Object%20Reference) (OtherActor :type Actor%20Object%20Reference) (OtherComp :type Primitive%20Component%20Object%20Reference) (OtherBodyIndex :type Integer) (bFromSweep :type Boolean) (SweepResult :type Hit%20Result%20Structure%20%28by%20ref%29))
  (if (Math|Boolean|ORBoolean (Actor|ActorHasTag OtherActor "Energy") (Actor|ActorHasTag OtherActor "Punch") (Actor|ActorHasTag OtherActor "EnemyBullet") (Actor|ActorHasTag OtherActor "Laser") (and (Actor|ActorHasTag OtherActor "Enemy") (not (Actor|ActorHasTag OtherActor "Robber"))))
    (bind _output_get (Variables|Default|SetHealth (- (Variables|Default|GetHealth) 1)))
    (if (<= _output_get 0)
      (Niagara|SpawnSystematLocation "/Game/Blueprints/ParticleSystem/Explosion.Explosion" (Transformation|GetWorldLocation (Variables|Default|GetBusMesh)) "91.000000,0.000000,0.000000")
      (Utilities|FlowControl|Delay 1.5)
      (Variables|Default|SetDistanceAlongSpline 0.0)
      (Variables|Default|SetHealth (Variables|Default|GetMaxHealth))
      (Rendering|SetVisibility (Variables|Default|GetSmoke) false false)
      (Transformation|SetActorTransform (Variables|Default|GetstartingTransform))
      (Variables|Default|SetcanMove true)
      (else
        (for _index (range 0 (Math|Random|RandomIntegerinRange 1 5))
          (Game|SpawnActorfromClass "/Game/Blueprints/Shrapnel/Shrapnel7.Shrapnel7_C" (Transformation|GetWorldTransform (Variables|Default|GetBusMesh)) "AdjustIfPossibleButAlwaysSpawn" "MultiplyWithRoot" 0 0)
          (if (<= (Variables|Default|GetHealth) 2)
            (Rendering|SetVisibility (Variables|Default|GetSmoke) true false)
            (if (<= (Variables|Default|GetHealth) 1)
              (Variables|Default|SetcanMove false))))))))

(event OnComponentEndOverlap(FrontSensor)
  (params (OverlappedComponent :type Primitive%20Component%20Object%20Reference) (OtherActor :type Actor%20Object%20Reference) (OtherComp :type Primitive%20Component%20Object%20Reference) (OtherBodyIndex :type Integer))
  (if (== (Math|Boolean|ANDBoolean (Actor|ActorHasTag OtherActor "Player") (Actor|ActorHasTag OtherActor "Enemy") (Actor|ActorHasTag OtherActor "Vehicle") (Actor|ActorHasTag OtherActor "Person")) false)
    (Variables|Default|SetcanMove true)))

(event OnComponentBeginOverlap(FrontSensor)
  (params (OverlappedComponent :type Primitive%20Component%20Object%20Reference) (OtherActor :type Actor%20Object%20Reference) (OtherComp :type Primitive%20Component%20Object%20Reference) (OtherBodyIndex :type Integer) (bFromSweep :type Boolean) (SweepResult :type Hit%20Result%20Structure%20%28by%20ref%29))
  (if (and (Math|Boolean|ORBoolean (Actor|ActorHasTag OtherActor "Player") (Actor|ActorHasTag OtherActor "Enemy") (Actor|ActorHasTag OtherActor "Vehicle") (Actor|ActorHasTag OtherActor "Person")) (!= OtherActor self))
    (Variables|Default|SetcanMove false)))

(event EventBeginPlay
  (Utilities|FlowControl|Sequence
    (:then_0
      (Rendering|Material|SetMaterial (Variables|Default|GetBusMesh) 0 (Utilities|Array|Get(acopy) (Utilities|Array|MakeArray (Variables|Default|Getcar1) (Variables|Default|Getcar1_0) (Variables|Default|Getcar1_1)) (Math|Random|RandomIntegerinRange 0 2))))
    (:then_1
      (Variables|Default|SetstartingTransform (Transformation|GetRelativeTransform (Variables|Character|GetMesh)))
      (Variables|Default|SetcanMove true))))

(event EventTick
  (params (DeltaSeconds :type Float%20%28single-precision%29))
  (if (and (Variables|Default|GetcanMove) (> (Variables|Default|GetHealth) 1))
    (Variables|Default|SetDistanceAlongSpline (+ (* DeltaSeconds (Variables|Default|GetSplineSpeed)) (Variables|Default|GetDistanceAlongSpline)))
    (Transformation|SetRelativeTransform (Variables|Default|GetBusMesh) (Math|Transform|MakeTransform (Math|Vector|MakeVector (.x (.location (Spline|GetTransformatDistanceAlongSpline (Variables|Default|GetSpline) (Variables|Default|GetDistanceAlongSpline) "World" false))) (.y (.location (Spline|GetTransformatDistanceAlongSpline (Variables|Default|GetSpline) (Variables|Default|GetDistanceAlongSpline) "World" false))) (.z (.location (Spline|GetTransformatDistanceAlongSpline (Variables|Default|GetSpline) (Variables|Default|GetDistanceAlongSpline) "World" false)))) (Math|Rotator|MakeRotator (.roll (.rotation (Spline|GetTransformatDistanceAlongSpline (Variables|Default|GetSpline) (Variables|Default|GetDistanceAlongSpline) "World" false))) (.pitch (.rotation (Spline|GetTransformatDistanceAlongSpline (Variables|Default|GetSpline) (Variables|Default|GetDistanceAlongSpline) "World" false))) (+ (.yaw (.rotation (Spline|GetTransformatDistanceAlongSpline (Variables|Default|GetSpline) (Variables|Default|GetDistanceAlongSpline) "World" false))) -9e+01)) (Variables|/Script/Engine.SceneComponent|GetRelativeScale3D (Variables|Default|GetBusMesh))) false false)
    (if (Variables|Default|GetcanLoop)
      (if (> (Variables|Default|GetDistanceAlongSpline) (Spline|GetSplineLength (Variables|Default|GetSpline)))
        (Variables|Default|SetDistanceAlongSpline 0.0)))))

(event EventPickUp
  (Variables|Default|SetcanMove false))

(event EventRelease
  (Variables|Default|SetHealth 1)
  (Rendering|SetVisibility (Variables|Default|GetSmoke) true false))

(fn ConstructionScript)