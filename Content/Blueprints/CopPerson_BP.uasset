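; Cop pedestrian pawn, apparently built on civilian logic, that issues AI MoveTo toward a target destination every Tick.
; Enemy overlaps on its sphere switch states that set speed, while capsule hits and PickUp ragdoll the mesh.
; Functions for trace-based walking, sidewalk seeking, fleeing muggers and ragdoll recovery exist.
; The state dispatch calling them is disconnected, so that behavior, including getting up after Release, never runs.
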(event OnComponentHit(Capsule)
  (params (HitComponent :type Primitive%20Component%20Object%20Reference) (OtherActor :type Actor%20Object%20Reference) (OtherComp :type Primitive%20Component%20Object%20Reference) (NormalImpulse :type Vector :default "0, 0, 0") (Hit :type Hit%20Result%20Structure%20%28by%20ref%29))
  ;[1 1 1 0.2] Capsule Collision
  (CallFunction|Ragdoll true))

(event OnComponentBeginOverlap(Sphere)
  (params (OverlappedComponent :type Primitive%20Component%20Object%20Reference) (OtherActor :type Actor%20Object%20Reference) (OtherComp :type Primitive%20Component%20Object%20Reference) (OtherBodyIndex :type Integer) (bFromSweep :type Boolean) (SweepResult :type Hit%20Result%20Structure%20%28by%20ref%29))
  ;[1 1 1 0.2] Sphere Collision
  (Utilities|FlowControl|Sequence
    (:then_0
      (Utilities|Casting|CastToMugger_Enemy_BP OtherActor))
    (:then_1
      (Utilities|Casting|CastToSentry_Enemy_BP OtherActor))
    (:then_2
      (Utilities|Casting|CastToGround_Enemy_BP OtherActor)))
  (CallFunction|SetState 2))

(event OnComponentBeginOverlap(Capsule)
  (params (OverlappedComponent :type Primitive%20Component%20Object%20Reference) (OtherActor :type Actor%20Object%20Reference) (OtherComp :type Primitive%20Component%20Object%20Reference) (OtherBodyIndex :type Integer) (bFromSweep :type Boolean) (SweepResult :type Hit%20Result%20Structure%20%28by%20ref%29))
  ;[1 1 1 0.2] Capsule Collision
  (if (< (Variables|Default|GetState) 2)
    (Utilities|Casting|CastToSidewalk_BP OtherActor)))

(event OnComponentEndOverlap(Sphere)
  (params (OverlappedComponent :type Primitive%20Component%20Object%20Reference) (OtherActor :type Actor%20Object%20Reference) (OtherComp :type Primitive%20Component%20Object%20Reference) (OtherBodyIndex :type Integer))
  ;[1 1 1 0.2] Sphere Collision
  (Utilities|FlowControl|Sequence
    (:then_0
      (Utilities|Casting|CastToMugger_Enemy_BP OtherActor))
    (:then_1
      (Utilities|Casting|CastToSentry_Enemy_BP OtherActor))
    (:then_2
      (Utilities|Casting|CastToGround_Enemy_BP OtherActor)))
  (CallFunction|SetState))

(event Custom|ResetRagdoll
  (CallFunction|Ragdoll false)
  (CallFunction|ResettoMeshPosition))

(event EventBeginPlay
  (CallFunction|SetState 1)
  (Variables|Default|SetsetMesh 0)
  (Components|SkeletalMesh|SetSkeletalMeshAsset (Variables|Default|GetCityMan) (Variables|Default|GetWoman_Mesh)))

(event EventRelease
  (CallFunction|SetState 3))

(event EventPickUp
  (Utilities|Time|ClearTimerbyFunctionName 0 "ResetRagdoll")
  (CallFunction|Ragdoll true)
  (CallFunction|SetState 4))

(event EventTick
  (params (DeltaSeconds :type Float%20%28single-precision%29))
  (Utilities|FlowControl|Sequence
    (:then_1
      (AI|AIMoveTo self (Variables|Default|GetTarget%20Destination) 0 5.0 false))))

(fn ConstructionScript)

(fn Ragdoll
  (params (IsRagdoll :type Boolean))
  (bind _capsule (Variables|Default|GetCapsule))
  (bind _cityman (Variables|Default|GetCityMan))
  (if IsRagdoll
    (Collision|SetCollisionProfileName _capsule "NoCollision" true :!class /Script/Engine.PrimitiveComponent)
    (Audio|Components|Audio|Stop _cityman)
    (Physics|SetSimulatePhysics _cityman true)
    (else
      (Physics|SetSimulatePhysics _cityman false)
      (Collision|SetCollisionProfileName _capsule "Pawn" true :!class /Script/Engine.PrimitiveComponent)
      (Audio|Components|Audio|Play _cityman false)))
  (CallFunction|SetState (Math|Integer|SelectInt 3 1 IsRagdoll))
  (return))

(fn MoveForward
  (params (DeltaTime :type Float%20%28double-precision%29))
  (bind _scene (Variables|Default|GetScene))
  (bind _scene_2 (Variables|Default|GetScene))
  (bind _returnvalue (Transformation|GetWorldLocation _scene_2))
  (bind (_outhit _returnvalue_2) (Collision|LineTraceByChannel _returnvalue (+ _returnvalue (Math|Vector|MakeVector 0.0 0.0 -1e+02)) "TraceTypeQuery1" false (Utilities|Array|MakeArray (Game|GetPlayerCharacter 0)) "None"))
  (if _returnvalue_2
    (Transformation|SetWorldLocation (Variables|Default|GetScene) (Math|Vector|SelectVector (+ (* (Variables|Default|GetSpeed) DeltaTime (Math|Vector|GetForwardVector _scene)) (Transformation|GetWorldLocation _scene) (Math|Vector|SelectVector (Math|Vector|VectorUp) (Math|Vector|VectorZero) (and (<= (.Distance (Collision|BreakHitResult _outhit)) 8e+01) (Utilities|Enum|Equal(Enum) (Variables|/Script/Engine.SceneComponent|GetMobility (.HitComponent (Collision|BreakHitResult _outhit))) "Static")))) "0, 0, 0" _returnvalue_2) false false)
    (else
      (Transformation|SetWorldLocation (Variables|Default|GetScene) (+ (Math|Vector|VectorDown) (Transformation|GetWorldLocation (Variables|Default|GetScene))) false false))))

(fn Lookat
  (params (StartTarget :type Vector) (LookTarget :type Vector))
  (Transformation|SetActorRotation (Math|Rotator|MakeRotator 0.0 0.0 (.yaw (Math|Rotator|FindLookatRotation StartTarget LookTarget)))))

(fn FindClosestActorSphere
  (params (ActorClassRef :type Actor%20Class%20Reference))
  (bind _self self)
  (bind _sphere (Variables|Default|GetSphere))
  (bind _overlappingactors (Collision|GetOverlappingActors _sphere ActorClassRef :!class /Script/Engine.PrimitiveComponent))
  (if (!= (Utilities|Array|Length _overlappingactors) 0)
    (for (_array_element _array_index) _overlappingactors
      (if (!= _array_index 0)
        (if (< (Transformation|GetDistanceTo _array_element _self) (Transformation|GetDistanceTo (LocalVariables|GetClosestClass) _self))
          (LocalVariables|SetClosestClass _array_element :!label _label))
        (else
          (goto _label))))
    (return (Transformation|GetActorLocation (LocalVariables|GetClosestClass)))
    (else
      (return (Transformation|GetActorLocation self)))))

(fn SetState
  (params (NewState :type Integer))
  (bind _output_get (Variables|Default|SetState NewState))
  (switch int _output_get
    (:0
      (Variables|Default|SetSpeed (Math|Float|SelectFloat 0.0 5e+01 (>= (Math|Random|RandomFloat) 0.8))))
    (:1
      (Variables|Default|SetSpeed 5e+01))
    (:2
      (Variables|Default|SetSpeed 1.5e+02))
    (:3
      (Variables|Default|SetSpeed 0.0))))

(fn IsSidewalk
  (bind _capsule (Variables|Default|GetCapsule))
  (bind _overlappingactors (Collision|GetOverlappingActors _capsule "/Game/Blueprints/Sidewalk_BP.Sidewalk_BP_C" :!class /Script/Engine.PrimitiveComponent))
  (if (Utilities|Array|IsNotEmpty _overlappingactors)
    (bind _assidewalk_bp (Utilities|Casting|CastToSidewalk_BP (Utilities|Array|Get(acopy) _overlappingactors))
      (:then
        (return true _assidewalk_bp))
      (:CastFailed
        _)))
  (return false 0))

(fn ResettoMeshPosition
  (bind _scene (Variables|Default|GetScene))
  (bind _cityman (Variables|Default|GetCityMan))
  (bind _cityman_2 (Variables|Default|GetCityMan))
  (bind _returnvalue (Transformation|GetWorldTransform _scene))
  (bind _returnvalue_2 (Transformation|GetWorldTransform _cityman))
  (Transformation|SetWorldLocationAndRotation _scene (Math|Vector|MakeVector (.x (.location _returnvalue_2)) (.y (.location _returnvalue_2)) (+ (.z (.location _returnvalue_2)) 85.0)) (Math|Rotator|MakeRotator (.roll (.rotation _returnvalue)) (.pitch (.rotation _returnvalue)) (.yaw (.rotation _returnvalue_2))) false true)
  (Transformation|AttachComponentToComponent _cityman_2 _scene "None" "SnapToTarget" "KeepRelative" "KeepRelative" false)
  (Transformation|SetRelativeLocationAndRotation _cityman_2 "0.000000,0.000000,-90.000000" "0.000000,-90.000000,0.000000" false false))

(fn CheckonGround
  (bind _cityman (Variables|Default|GetCityMan))
  (bind _returnvalue (Transformation|GetWorldLocation _cityman))
  (bind (_outhit _returnvalue_2) (Collision|LineTraceByChannel _returnvalue (+ _returnvalue (Math|Vector|MakeVector 0.0 0.0 -1e+02)) "TraceTypeQuery1" false (Utilities|Array|MakeArray (Game|GetPlayerCharacter 0)) "ForOneFrame"))
  (if _returnvalue_2
    (return (Utilities|Enum|Equal(Enum) (Variables|/Script/Engine.SceneComponent|GetMobility (.HitComponent (Collision|BreakHitResult _outhit))) "Static"))
    (else
      (return false))))