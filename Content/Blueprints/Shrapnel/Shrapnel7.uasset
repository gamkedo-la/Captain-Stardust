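; Shrapnel7 is a short-lived debris actor that appears as a randomly shaped shatter fragment.
; On BeginPlay it gives its Cube component a random scale per axis, enables gravity and swaps in a random mesh from a set of Shatter meshes.
; After a random delay of a few seconds it destroys itself, and its construction script is empty.
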(event EventBeginPlay
  (Transformation|SetRelativeScale3D (Variables|Default|GetCube) (Math|Vector|MakeVector (Math|Random|RandomFloatinRange 0.3 0.5) (Math|Random|RandomFloatinRange 0.3 0.5) (Math|Random|RandomFloatinRange 0.3 0.5)))
  (Physics|SetEnableGravity (Variables|Default|GetCube) true)
  (Components|StaticMesh|SetStaticMesh (Variables|Default|GetCube) (.OutItem (Utilities|Array|Random (Utilities|Array|MakeArray (Variables|Default|GetShatter1) (Variables|Default|GetShatter2) (Variables|Default|GetShatter3) (Variables|Default|GetShatter4) (Variables|Default|GetShatter5) (Variables|Default|GetShatter6) (Variables|Default|GetShatter7) (Variables|Default|GetShatter8) (Variables|Default|GetShatter9) (Variables|Default|GetShatter10) (Variables|Default|GetShatter11) (Variables|Default|GetShatter12) (Variables|Default|GetShatter13)))))
  (Utilities|FlowControl|Delay (Math|Random|RandomFloatinRange 2.0 5.0))
  (Actor|DestroyActor))

(fn ConstructionScript)