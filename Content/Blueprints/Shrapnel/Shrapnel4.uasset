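; Shrapnel actor that spawns as a short-lived, randomly shaped piece of debris.
; On BeginPlay, its Cube component gets a random scale on each axis, gravity and a mesh picked at random from a set of shatter meshes.
; It then adds an audio component using the Cube's relative transform and destroys itself after a brief random delay.
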(event EventBeginPlay
  (bind _cube (Variables|Default|GetCube))
  (Transformation|SetRelativeScale3D (Variables|Default|GetCube) (Math|Vector|MakeVector (Math|Random|RandomFloatinRange 0.15 0.3) (Math|Random|RandomFloatinRange 0.15 0.3) (Math|Random|RandomFloatinRange 0.15 0.3)))
  (Physics|SetEnableGravity (Variables|Default|GetCube) true)
  (Components|StaticMesh|SetStaticMesh _cube (.OutItem (Utilities|Array|Random (Utilities|Array|MakeArray (Variables|Default|GetShatter1) (Variables|Default|GetShatter2) (Variables|Default|GetShatter3) (Variables|Default|GetShatter4) (Variables|Default|GetShatter5) (Variables|Default|GetShatter6) (Variables|Default|GetShatter7) (Variables|Default|GetShatter8) (Variables|Default|GetShatter9) (Variables|Default|GetShatter10) (Variables|Default|GetShatter11) (Variables|Default|GetShatter12) (Variables|Default|GetShatter13)))))
  (AddComponent|AddAudioComponent false (Transformation|GetRelativeTransform _cube))
  (Utilities|FlowControl|Delay (Math|Random|RandomFloatinRange 0.5 3.0))
  (Actor|DestroyActor))

(fn ConstructionScript)