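; World event trigger zone that fires a random world event after the player stays inside its sphere for a random delay.
; Entering the sphere with a Player-tagged actor rolls a countdown between MinTime and MaxTime, which Tick decrements until it fires once.
; Leaving halts the countdown, and re-entering rolls a new one.
; The three possible events are placeholders that only print debug strings.
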(event OnComponentBeginOverlap(Sphere)
  (params (OverlappedComponent :type Primitive%20Component%20Object%20Reference) (OtherActor :type Actor%20Object%20Reference) (OtherComp :type Primitive%20Component%20Object%20Reference) (OtherBodyIndex :type Integer) (bFromSweep :type Boolean) (SweepResult :type Hit%20Result%20Structure%20%28by%20ref%29))
  ;[1 1 1] Player Entered Zone
  (if (Actor|ActorHasTag (stale OnComponentEndOverlap(Sphere) OtherActor) "Player")
    (Variables|Default|SetplayerIsInArea true)
    (bind _output_get (Variables|Default|SetcurrentTime (Math|Random|RandomFloatinRange (Variables|Default|GetminTime) (Variables|Default|GetmaxTime))))
    (Development|PrintString "PlayerEnteredZone")
    (Development|PrintString (Utilities|String|ToString(Float) _output_get))))

(event OnComponentEndOverlap(Sphere)
  (params (OverlappedComponent :type Primitive%20Component%20Object%20Reference) (OtherActor :type Actor%20Object%20Reference) (OtherComp :type Primitive%20Component%20Object%20Reference) (OtherBodyIndex :type Integer))
  ;[1 1 1] Player Left Zone
  (if (Actor|ActorHasTag OtherActor "Player")
    (Variables|Default|SetplayerIsInArea false)
    (Development|PrintString "PlayerLeftWorldEvent")))

(event Custom|TriggerWorldEvent
  ;[1 1 1] Create World Event
  (switch int (Math|Random|RandomInteger 3)
    (:0
      (Development|PrintString "World Event 1"))
    (:1
      (Development|PrintString "World Event 2"))
    (:2
      (Development|PrintString "World Event 3"))))

(event EventTick
  (params (DeltaSeconds :type Float%20%28single-precision%29))
  ;[1 1 1] Countdown Timer of WorldEvent
  (if (Variables|Default|GetplayerIsInArea)
    (if (> (Variables|Default|GetcurrentTime) 0.0)
      (Variables|Default|SetcurrentTime (- (Variables|Default|GetcurrentTime) (Utilities|Time|GetWorldDeltaSeconds)))
      (else
        (CallFunction|TriggerWorldEvent)
        (Variables|Default|SetplayerIsInArea false)))))

(fn ConstructionScript)