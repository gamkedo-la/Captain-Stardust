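; CityMan is a city character actor that walks forward at Speed every Tick and gets knocked down when its capsule is hit.
; Knockdown briefly ragdolls the mesh with capsule collision off, then restores both.
; To recover, it moves the root to the mesh's X/Y and yaw, keeping its own height, then reattaches the mesh.
; Idle/walking state cycling and debug prints are present but unconnected.
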(event OnComponentHit(Capsule)
  (params (HitComponent :type Primitive%20Component%20Object%20Reference) (OtherActor :type Actor%20Object%20Reference) (OtherComp :type Primitive%20Component%20Object%20Reference) (NormalImpulse :type Vector :default "0, 0, 0") (Hit :type Hit%20Result%20Structure%20%28by%20ref%29))
  (CallFunction|Knockdown))

(event Custom|Knockdown
  (bind _cityman (Variables|Default|GetCityMan))
  (bind _defaultsceneroot (Variables|Default|GetDefaultSceneRoot))
  (bind _cityman_2 (Variables|Default|GetCityMan))
  (bind _returnvalue (Transformation|GetWorldTransform _defaultsceneroot))
  (bind _returnvalue_2 (Transformation|GetWorldTransform _cityman))
  (CallFunction|Ragdoll true)
  (Utilities|FlowControl|Delay 1.0)
  (CallFunction|Ragdoll false)
  ;[1 1 1] Reset Position to Mesh's Position
  (Transformation|SetWorldLocationAndRotation _defaultsceneroot (Math|Vector|MakeVector (.x (.location _returnvalue_2)) (.y (.location _returnvalue_2)) (.z (.location _returnvalue))) (Math|Rotator|MakeRotator (.roll (.rotation _returnvalue)) (.pitch (.rotation _returnvalue)) (.yaw (.rotation _returnvalue_2))) false false)
  (Transformation|AttachComponentToComponent _cityman_2 _defaultsceneroot "None" "KeepRelative" "KeepRelative" "KeepRelative" true)
  (Transformation|SetRelativeLocationAndRotation _cityman_2 "0.000000,0.000000,0.000000" "0.000000,-90.000000,0.000000" false false))

(event EventBeginPlay)

(event EventTick
  (params (DeltaSeconds :type Float%20%28single-precision%29))
  (bind _defaultsceneroot (Variables|Default|GetDefaultSceneRoot))
  (Transformation|SetWorldLocation _defaultsceneroot (+ (* DeltaSeconds (* (Variables|Default|GetSpeed) (Math|Vector|GetForwardVector _defaultsceneroot))) (Transformation|GetWorldLocation _defaultsceneroot)) false false))

(fn ConstructionScript)

(fn Ragdoll
  (params (IsRagdoll :type Boolean))
  (bind _capsule (Variables|Default|GetCapsule))
  (Physics|SetSimulatePhysics (Variables|Default|GetCityMan) IsRagdoll)
  (if IsRagdoll
    (Collision|SetCollisionEnabled _capsule "NoCollision")
    (else
      (Collision|SetCollisionEnabled _capsule "QueryAndPhysics")))
  (return))