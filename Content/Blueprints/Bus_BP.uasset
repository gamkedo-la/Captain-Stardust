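; Bus_BP is a destructible bus that takes damage from overlaps with actors tagged Enemy.
; On BeginPlay it gives the bus mesh one of three car materials at random.
; Each hit lowers Health by one and spawns a random handful of shrapnel actors, revealing smoke when health runs low.
; At zero health it spawns an explosion particle system and destroys itself.
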(event OnComponentBeginOverlap(BusMesh)
  (params (OverlappedComponent :type Primitive%20Component%20Object%20Reference) (OtherActor :type Actor%20Object%20Reference) (OtherComp :type Primitive%20Component%20Object%20Reference) (OtherBodyIndex :type Integer) (bFromSweep :type Boolean) (SweepResult :type Hit%20Result%20Structure%20%28by%20ref%29))
  (if (Actor|ActorHasTag OtherActor "Enemy")
    (bind _output_get (Variables|Default|SetHealth (- (Variables|Default|GetHealth) 1)))
    (if (<= _output_get 0)
      (Niagara|SpawnSystematLocation "/Game/Blueprints/ParticleSystem/Explosion.Explosion" (Transformation|GetWorldLocation (Variables|Default|GetBusMesh)) "0.000000,0.000000,-90.000000")
      (Actor|DestroyActor)
      (else
        (for _index (range 0 (Math|Random|RandomIntegerinRange 1 5))
          (Game|SpawnActorfromClass "/Game/Blueprints/Shrapnel/Shrapnel7.Shrapnel7_C" (Transformation|GetActorTransform) "AdjustIfPossibleButAlwaysSpawn" "MultiplyWithRoot" 0 0)
          (if (<= (Variables|Default|GetHealth) 2)
            (Rendering|SetVisibility (Variables|Default|GetSmoke) true false)))))))

(event EventBeginPlay
  (Rendering|Material|SetMaterial (Variables|Default|GetBusMesh) 0 (Utilities|Array|Get(acopy) (Utilities|Array|MakeArray (Variables|Default|Getcar1) (Variables|Default|Getcar1_0) (Variables|Default|Getcar1_1)) (Math|Random|RandomIntegerinRange 0 2))))

(fn ConstructionScript)