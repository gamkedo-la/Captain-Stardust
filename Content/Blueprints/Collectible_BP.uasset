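; Collectible pickup actor that spins at SpinRate and counts toward the player's collect total.
; When an actor tagged Player overlaps its static mesh, it increments the collect count on the player's BP_ThirdPersonCharacter, plays a 2D sound and destroys itself.
; Its minimap component is deactivated on BeginPlay, and a RemoveTickPrerequisiteComponent call is made on it before destruction.
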(event OnComponentBeginOverlap(StaticMesh)
  (params (OverlappedComponent :type Primitive%20Component%20Object%20Reference) (OtherActor :type Actor%20Object%20Reference) (OtherComp :type Primitive%20Component%20Object%20Reference) (OtherBodyIndex :type Integer) (bFromSweep :type Boolean) (SweepResult :type Hit%20Result%20Structure%20%28by%20ref%29))
  (if (Actor|ActorHasTag OtherActor "Player")
    (bind _asbp_third_person_character (Utilities|Casting|CastToBP_ThirdPersonCharacter (Game|Player|GetPlayerPawn 0)))
    (Default|IncreaseCollectCount _asbp_third_person_character)
    (Audio|PlaySound2D "/Game/Audio/ComicSound.ComicSound" 1.0 1.0 0.0 0 0)
    (Class|ActorComponent|RemoveTickPrerequisiteComponent (Variables|Default|GetBP_Minimap_Component))
    (Actor|DestroyActor)))

(event EventBeginPlay
  (Components|Activation|SetActive (Variables|Default|GetBP_Minimap_Component) false false))

(event Collision|EventActorBeginOverlap
  (params (OtherActor :type Actor%20Object%20Reference)))

(event EventTick
  (params (DeltaSeconds :type Float%20%28single-precision%29))
  (Transformation|AddLocalRotation (Variables|Default|GetStaticMesh) (Math|Rotator|MakeRotator 0.0 0.0 (* DeltaSeconds (Variables|Default|GetspinRate))) false false))

(fn ConstructionScript)