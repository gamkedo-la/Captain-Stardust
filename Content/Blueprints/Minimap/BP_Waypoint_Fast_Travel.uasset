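; Fast travel waypoint actor for the minimap that becomes discovered when the player walks into its box trigger.
; BeginPlay sets the MapIconBP icon's activation from HasDiscovered.
; A box overlap by BP_ThirdPersonCharacter calls Discover, which acts only once, setting the flag, activating the icon and hiding the mesh from scene captures.
; The travel itself is not handled in this graph.
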(event OnComponentBeginOverlap(Box)
  (params (OverlappedComponent :type Primitive%20Component%20Object%20Reference) (OtherActor :type Actor%20Object%20Reference) (OtherComp :type Primitive%20Component%20Object%20Reference) (OtherBodyIndex :type Integer) (bFromSweep :type Boolean) (SweepResult :type Hit%20Result%20Structure%20%28by%20ref%29))
  (Utilities|Casting|CastToBP_ThirdPersonCharacter OtherActor)
  (CallFunction|Discover))

(event EventBeginPlay
  (|CallParentFunction)
  (Default|ActivateIcon (Variables|Default|GetMapIcon_BP) (Variables|Default|GetHasDiscovered)))

(event Collision|EventActorBeginOverlap
  (params (OtherActor :type Actor%20Object%20Reference))
  (|CallParentFunction OtherActor) ; This node is disabled and will not be called.\nDrag off pins to build functionality.
)

(event EventTick
  (params (DeltaSeconds :type Float%20%28single-precision%29))
  (|CallParentFunction DeltaSeconds) ; This node is disabled and will not be called.\nDrag off pins to build functionality.
)

(event EventUpdateIconPosition
  (params (position :type Vector%202D%20Structure)))

(fn ConstructionScript
  (|CallParentFunction))

(fn Discover
  (if (not (Variables|Default|GetHasDiscovered))
    (bind _output_get (Variables|Default|SetHasDiscovered true))
    (Default|ActivateIcon (Variables|Default|GetMapIcon_BP) _output_get)
    (Class|PrimitiveComponent|SetHiddeninSceneCapture (Variables|Default|GetMesh) _output_get)))