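; BP_Waypoint is a world marker that shows its icon on the minimap, with the same icon as its billboard sprite.
; Shortly after BeginPlay it creates a minimap icon widget and attaches its CalcHelper component to the player's root.
; Each tick it moves CalcHelper to the waypoint's location, using the resulting relative location as a player-space 2D offset to position the icon without manual transform math.
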(event EventBeginPlay
  (Utilities|FlowControl|Delay 0.5)
  (bind _returnvalue (UserInterface|CreateWidget "/Game/Blueprints/Minimap/wdg_minimap_icon.wdg_minimap_icon_C"))
  (bind _output_get (Variables|Default|Setminimap_icon _returnvalue))
  (Default|ChangeIcon _output_get (Variables|Default|Geticon))
  (UserInterface|Viewport|AddtoViewport _output_get 0)
  (Transformation|AttachComponentToComponent (Variables|Default|Getcalc_helper) (Variables|/Script/Engine.Actor|GetRootComponent (Game|GetPlayerCharacter 0)) "None" "KeepWorld" "KeepWorld" "KeepWorld" true)
  (CallFunction|UpdateIconPosition))

(event Collision|EventActorBeginOverlap
  (params (OtherActor :type Actor%20Object%20Reference)))

(event EventTick
  (params (DeltaSeconds :type Float%20%28single-precision%29))
  (CallFunction|UpdateIconPosition))

(fn ConstructionScript
  (Rendering|Components|Sprite|SetSprite (Variables|Default|GetBillboard) (Variables|Default|Geticon)))

(fn UpdateIconPosition
  (Transformation|SetWorldLocation (Variables|Default|Getcalc_helper) (Transformation|GetActorLocation) false false)
  (bind _minimap_icon (Variables|Default|Getminimap_icon)
    (:then
      (Default|UpdateIconPos _minimap_icon (Math|Conversions|ToVector2D(Vector) (Variables|/Script/Engine.SceneComponent|GetRelativeLocation (Variables|Default|Getcalc_helper)))))
    (:else)))