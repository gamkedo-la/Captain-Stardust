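; Minimap actor that puts the minimap widget on screen and feeds it the player's position and heading.
; BeginPlay creates Wdg_minimap and adds it to the viewport.
; Every Tick writes player location and control yaw to the MP_Minimap Material Parameter Collection, so materials can read them.
; The yaw is offset by 270 degrees, wrapped if negative, and divided by 360 to express it as a fraction of a turn.
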(event EventBeginPlay
  (bind _returnvalue (UserInterface|CreateWidget "/Game/Blueprints/Minimap/wdg_minimap.wdg_minimap_C"))
  (UserInterface|Viewport|AddtoViewport _returnvalue 0))

(event Collision|EventActorBeginOverlap
  (params (OtherActor :type Actor%20Object%20Reference)))

(event EventTick
  (params (DeltaSeconds :type Float%20%28single-precision%29))
  (bind _returnvalue (Game|GetPlayerController 0))
  (bind _returnvalue_2 (Pawn|GetControlRotation _returnvalue :!class /Script/Engine.Controller))
  (bind _yaw (Math|Rotator|BreakRotator _returnvalue_2))
  (bind _returnvalue_3 (- _yaw 2.7e+02))
  (Rendering|Material|SetVectorParameterValue "/Game/Blueprints/Minimap/MP_Minimap.MP_Minimap" "Player Location" (Math|Conversions|ToLinearColor(Vector) (Transformation|GetActorLocation (Game|GetPlayerCharacter 0))) :!class /Script/Engine.KismetMaterialLibrary)
  (Rendering|Material|SetScalarParameterValue "/Game/Blueprints/Minimap/MP_Minimap.MP_Minimap" "Player Yaw" (/ (Math|Float|SelectFloat (+ _returnvalue_3 3.6e+02) _returnvalue_3 (< _returnvalue_3 0.0)) 3.6e+02) :!class /Script/Engine.KismetMaterialLibrary))

(fn ConstructionScript)