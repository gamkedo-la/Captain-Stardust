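; Actor component that shows its owner as an icon on the minimap.
; Shortly after BeginPlay it creates the icon widget and adds a helper scene component attached to the player character's root.
; Each tick it moves the helper to the owner's world location and feeds its relative location to the icon as a 2D player-space offset, avoiding manual transform math.
; EndPlay deletes the icon.
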(event EventBeginPlay
  (Utilities|FlowControl|Delay 0.5)
  (bind _returnvalue (UserInterface|CreateWidget "/Game/Blueprints/Minimap/wdg_minimap_icon.wdg_minimap_icon_C"))
  (bind _output_get (Variables|Default|Setminimap_icon _returnvalue))
  (Default|ChangeIcon _output_get (Variables|Default|Geticon))
  (UserInterface|Viewport|AddtoViewport _output_get 0)
  (bind _returnvalue_2 (Game|AddComponentbyClass (Components|GetOwner) "/Script/Engine.SceneComponent" false))
  (bind _output_get_2 (Variables|Default|Setcalc_helper _returnvalue_2))
  (Transformation|AttachComponentToComponent _output_get_2 (Variables|/Script/Engine.Actor|GetRootComponent (Game|GetPlayerCharacter 0)) "None" "KeepWorld" "KeepWorld" "KeepWorld" true))

(event EventTick
  (params (DeltaSeconds :type Float%20%28single-precision%29))
  (CallFunction|UpdateIconPosition))

(event EventEndPlay
  (params (EndPlayReason :type EEndPlayReason%20Enum :default "Destroyed"))
  (Default|DeleteIcon (Variables|Default|Getminimap_icon)))

(fn UpdateIconPosition
  (bind _calc_helper (Variables|Default|Getcalc_helper)
    (:then
      (Transformation|SetWorldLocation _calc_helper (Transformation|GetActorLocation (Components|GetOwner)) false false)
      (bind _minimap_icon (Variables|Default|Getminimap_icon)
        (:then
          (Default|UpdateIconPos _minimap_icon (Math|Conversions|ToVector2D(Vector) (Variables|/Script/Engine.SceneComponent|GetRelativeLocation (Variables|Default|Getcalc_helper)))))
        (:else)))
    (:else)))