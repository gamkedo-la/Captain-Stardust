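; Laser actor that bursts into shrapnel when it hits a building, and otherwise destroys itself after a short delay.
; Its Cylinder overlap checks for the Building tag, spawns a random number of Shrapnel1 actors in three tiers by the laser's X scale, then destroys the laser.
; An unconnected House branch, which would spawn the house's own shrapnel class, never runs.
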(event OnComponentBeginOverlap(Cylinder)
  (params (OverlappedComponent :type Primitive%20Component%20Object%20Reference) (OtherActor :type Actor%20Object%20Reference) (OtherComp :type Primitive%20Component%20Object%20Reference) (OtherBodyIndex :type Integer) (bFromSweep :type Boolean) (SweepResult :type Hit%20Result%20Structure%20%28by%20ref%29))
  ;[1 1 1] Hit Building Collision
  (if (Actor|ActorHasTag OtherActor "Building")
    (if (<= (.x (Transformation|GetActorScale3D)) 0.2)
      (for _index (range 0 (Math|Random|RandomIntegerinRange 1 5))
        (Game|SpawnActorfromClass "/Game/Blueprints/Shrapnel/Shrapnel1.Shrapnel1_C" (Transformation|GetActorTransform) "Undefined" "MultiplyWithRoot" 0 0))
      (elif (< (.x (Transformation|GetActorScale3D)) 0.5)
        (for _index_2 (range 0 (Math|Random|RandomIntegerinRange 5 15))
          (Game|SpawnActorfromClass "/Game/Blueprints/Shrapnel/Shrapnel1.Shrapnel1_C" (Transformation|GetActorTransform) "Undefined" "MultiplyWithRoot" 0 0))
        (else
          (for _index_3 (range 0 (Math|Random|RandomIntegerinRange 15 30))
            (Game|SpawnActorfromClass "/Game/Blueprints/Shrapnel/Shrapnel1.Shrapnel1_C" (Transformation|GetActorTransform) "Undefined" "MultiplyWithRoot" 0 0)))))
    (Actor|DestroyActor)))

(event EventBeginPlay
  (Utilities|FlowControl|Delay 4.0)
  (Actor|DestroyActor))

(fn ConstructionScript)