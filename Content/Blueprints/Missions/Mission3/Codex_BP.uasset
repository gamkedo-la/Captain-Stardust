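; Mission 3 Codex pickup that the player delivers to Mission Control, advancing the objective when first picked up.
; PickUp sets mesh physics simulation from the carry flag and, the first time only, replaces objective widgets and starts Prof D's narration.
; After a delay following that dialog's start, it spawns the Mission 3 delivery actor at a fixed location.
; Tick teleports the Codex to a fixed position if it falls below a height threshold.
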(event EventBeginPlay
  (|CallParentFunction) ; This node is disabled and will not be called.\nDrag off pins to build functionality.
)

(event Collision|EventActorBeginOverlap
  (params (OtherActor :type Actor%20Object%20Reference))
  (|CallParentFunction OtherActor) ; This node is disabled and will not be called.\nDrag off pins to build functionality.
)

(event EventTick
  (params (DeltaSeconds :type Float%20%28single-precision%29))
  (|CallParentFunction DeltaSeconds)
  (if (<= (.z (.location (Transformation|GetActorTransform))) -2e+02)
    (Transformation|SetActorTransform (Math|Transform|MakeTransform "1880.000000,2280.000000,2188.000000" "0.000000,0.000000,0.000000" "1.000000,1.000000,1.000000"))))

(event EventPickUp
  (bind _output_get (Variables|Default|SetIsBeingCarry (Variables|Default|GetIs%20Being%20Carry)))
  (Physics|SetSimulatePhysics (Variables|Character|GetMesh) _output_get)
  (if (Variables|Default|GetPickedUpFirstTime)
    (Development|PrintString "already picked up")
    (else
      (Variables|Default|SetPickedUpFirstTime true)
      ;[1 1 1] Updating Obective once player reaches the box
      (bind _foundwidgets (Widget|GetAllWidgetsOfClass "/Game/Blueprints/Widgets/Objective_Widget.Objective_Widget_C" true))
      (for _array_element _foundwidgets
        (Widget|SetVisibility _array_element "Hidden"))
      (bind _returnvalue (UserInterface|CreateWidget "/Game/Blueprints/Widgets/Objective_Widget.Objective_Widget_C"))
      (UserInterface|Viewport|AddtoViewport _returnvalue 0)
      (Default|UpdateObjective _returnvalue "Sentinel Surge")
      (Default|UpdateObjectiveText _returnvalue "Deliver Codex to Mission Control")
      ;[1 1 1] Spawn Dialog for entering level
      (bind _returnvalue_2 (Game|SpawnActorfromClass "/Game/Blueprints/Narration_Text_BP.Narration_Text_BP_C" (Math|Transform|MakeTransform "0, 0, 0" "0, 0, 0" "1.000000,1.000000,1.000000") "Undefined" "MultiplyWithRoot" 0 0))
      (Variables|/Game/Blueprints/Narration_Text_BP.Narration_Text_BP_C|SetCharacterNameArray _returnvalue_2 (Utilities|Array|MakeArray "Prof D" "Prof D" "Prof D"))
      (Variables|/Game/Blueprints/Narration_Text_BP.Narration_Text_BP_C|SetCharacterTextArray _returnvalue_2 (Utilities|Array|MakeArray "Most intriguing..." "The Codex you have contains the location of where these aliens came from. " "Once you deliver it, I am going to need to study it for a while to crack it to reveal their information."))
      (Variables|/Game/Blueprints/Narration_Text_BP.Narration_Text_BP_C|SetTimeDelay _returnvalue_2 (Utilities|Array|MakeArray 3.0 4.0 5.0))
      (Variables|/Game/Blueprints/Narration_Text_BP.Narration_Text_BP_C|SetIncrementSystem _returnvalue_2 -1)
      (bind _returnvalue_3 (UserInterface|CreateWidget "/Game/Blueprints/Widgets/NarrativeText_Blueprint.NarrativeText_Blueprint_C"))
      (UserInterface|Viewport|AddtoViewport _returnvalue_3 0)
      (Default|StartDialog _returnvalue_2)
      (Utilities|FlowControl|Delay 12.0)
      (Game|SpawnActorfromClass "/Game/Blueprints/Missions/Mission3/Delivery_BP_Mission3.Delivery_BP_Mission3_C" (Math|Transform|MakeTransform "3000.000000,14300.000000,900.000000" "0, 0, 0" "1.000000,1.000000,1.000000") "Undefined" "MultiplyWithRoot" 0 0))))

(fn ConstructionScript
  (|CallParentFunction))