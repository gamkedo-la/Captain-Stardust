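; Mission 2 dossier pickup that advances the mission the first time the player picks it up.
; PickUp flags it as carried and enables mesh physics on every call.
; The first pickup hides existing objective widgets and shows a new one with the mission name and description.
; It also spawns three sentry enemies offset from the mesh's relative location, plus two checkpoint triggers and the delivery point at hardcoded locations.
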(event EventBeginPlay
  (|CallParentFunction) ; This node is disabled and will not be called.\nDrag off pins to build functionality.
)

(event Collision|EventActorBeginOverlap
  (params (OtherActor :type Actor%20Object%20Reference))
  (|CallParentFunction OtherActor) ; This node is disabled and will not be called.\nDrag off pins to build functionality.
)

(event EventTick
  (params (DeltaSeconds :type Float%20%28single-precision%29))
  (|CallParentFunction DeltaSeconds))

(event EventPickUp
  (bind _output_get (Variables|Default|SetIsBeingCarry true))
  (Physics|SetSimulatePhysics (Variables|Character|GetMesh) _output_get)
  (if (Variables|Default|GetPickedUpFirstTime)
    (Development|PrintString "already picked up")
    (else
      (Development|PrintString "Start Timer")
      (Variables|Default|SetPickedUpFirstTime true)
      ;[1 1 1] Updating Obective once player reaches the box
      (bind _foundwidgets (Widget|GetAllWidgetsOfClass "/Game/Blueprints/Widgets/Objective_Widget.Objective_Widget_C" true))
      (for _array_element _foundwidgets
        (Widget|SetVisibility _array_element "Hidden"))
      (bind _returnvalue (UserInterface|CreateWidget "/Game/Blueprints/Widgets/Objective_Widget.Objective_Widget_C"))
      (UserInterface|Viewport|AddtoViewport _returnvalue 0)
      (Default|UpdateObjective _returnvalue (Variables|Default|GetMissionName))
      (Default|UpdateObjectiveText _returnvalue (Variables|Default|GetMissionDescription))
      ;[1 1 1] Spawn Enemies
      (Game|SpawnActorfromClass "/Game/Blueprints/Enemies/Sentry_Enemy_BP.Sentry_Enemy_BP_C" (Math|Transform|MakeTransform (+ (.location (Transformation|GetRelativeTransform (Variables|Character|GetMesh))) "-50.000000,-50.000000,50.000000") "0, 0, 0" "1.000000,1.000000,1.000000") "Undefined" "MultiplyWithRoot" 0 0)
      (Game|SpawnActorfromClass "/Game/Blueprints/Enemies/Sentry_Enemy_BP.Sentry_Enemy_BP_C" (Math|Transform|MakeTransform (+ (.location (Transformation|GetRelativeTransform (Variables|Character|GetMesh))) "30.000000,30.000000,30.000000") "0, 0, 0" "1.000000,1.000000,1.000000") "Undefined" "MultiplyWithRoot" 0 0)
      (Game|SpawnActorfromClass "/Game/Blueprints/Enemies/Sentry_Enemy_BP.Sentry_Enemy_BP_C" (Math|Transform|MakeTransform (+ (.location (Transformation|GetRelativeTransform (Variables|Character|GetMesh))) "0.000000,0.000000,60.000000") "0, 0, 0" "1.000000,1.000000,1.000000") "Undefined" "MultiplyWithRoot" 0 0)
      (Game|SpawnActorfromClass "/Game/Blueprints/Missions/Mission2/CheckpointTrigger_BP.CheckpointTrigger_BP_C" (Math|Transform|MakeTransform "1680.000000,1380.000000,2600.000000" "0, 0, 0" "1.000000,1.000000,1.000000") "Undefined" "MultiplyWithRoot" 0 0)
      (Game|SpawnActorfromClass "/Game/Blueprints/Missions/Mission2/CheckpointTrigger_BP.CheckpointTrigger_BP_C" (Math|Transform|MakeTransform "1680.000000,5300.000000,2600.000000" "0, 0, 0" "1.000000,1.000000,1.000000") "Undefined" "MultiplyWithRoot" 0 0)
      (Game|SpawnActorfromClass "/Game/Blueprints/Missions/Mission2/Delivery_BP_Mission2.Delivery_BP_Mission2_C" (Math|Transform|MakeTransform "2980.000000,14310.000000,860.000000" "0, 0, 0" "1.000000,1.000000,1.000000") "Undefined" "MultiplyWithRoot" 0 0))))

(fn ConstructionScript
  (|CallParentFunction))