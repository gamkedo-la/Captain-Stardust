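; One-shot checkpoint trigger for Mission 2 that saves the player's respawn point and springs an enemy ambush.
; When an actor tagged Player overlaps its Cube, it casts the player pawn to BP_ThirdPersonCharacter and calls StorePlayerRespawnPoint.
; It then spawns two Sentry_Enemy_BP actors at opposite diagonal world-space offsets from the player's location and destroys itself.
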(event OnComponentBeginOverlap(Cube)
  (params (OverlappedComponent :type Primitive%20Component%20Object%20Reference) (OtherActor :type Actor%20Object%20Reference) (OtherComp :type Primitive%20Component%20Object%20Reference) (OtherBodyIndex :type Integer) (bFromSweep :type Boolean) (SweepResult :type Hit%20Result%20Structure%20%28by%20ref%29))
  (if (Actor|ActorHasTag OtherActor "Player")
    (bind _asbp_third_person_character (Utilities|Casting|CastToBP_ThirdPersonCharacter (Game|Player|GetPlayerPawn 0)))
    (Default|StorePlayerRespawnPoint _asbp_third_person_character)
    (Game|SpawnActorfromClass "/Game/Blueprints/Enemies/Sentry_Enemy_BP.Sentry_Enemy_BP_C" (Math|Transform|MakeTransform (+ (.location (Transformation|GetActorTransform _asbp_third_person_character)) "-300.000000,-300.000000,50.000000") "0, 0, 0" "1.000000,1.000000,1.000000") "Undefined" "MultiplyWithRoot" 0 0)
    (Game|SpawnActorfromClass "/Game/Blueprints/Enemies/Sentry_Enemy_BP.Sentry_Enemy_BP_C" (Math|Transform|MakeTransform (+ (.location (Transformation|GetActorTransform _asbp_third_person_character)) "300.000000,300.000000,30.000000") "0, 0, 0" "1.000000,1.000000,1.000000") "Undefined" "MultiplyWithRoot" 0 0)
    (Actor|DestroyActor)))

(event EventBeginPlay)

(event Collision|EventActorBeginOverlap
  (params (OtherActor :type Actor%20Object%20Reference)))

(event EventTick
  (params (DeltaSeconds :type Float%20%28single-precision%29)))

(fn ConstructionScript)