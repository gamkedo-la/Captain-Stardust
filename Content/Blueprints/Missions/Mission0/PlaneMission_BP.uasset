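; PlaneMission_BP is an actor in Mission0, apparently for a plane, that resets itself when it drops too low.
; Every Tick it checks its world Z and, at or below a fixed negative height, sets its transform to a hard-coded location and rotation.
; BeginPlay and overlap events are disabled stubs, and the construction script only calls its parent.
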(event EventBeginPlay
  (|CallParentFunction) ; This node is disabled and will not be called.\nDrag off pins to build functionality.
)

(event Collision|EventActorBeginOverlap
  (params (OtherActor :type Actor%20Object%20Reference))
  (|CallParentFunction OtherActor) ; This node is disabled and will not be called.\nDrag off pins to build functionality.
)

(event EventTick
  (params (DeltaSeconds :type Float%20%28single-precision%29))
  (|CallParentFunction DeltaSeconds)
  (if (<= (.z (.location (Transformation|GetActorTransform))) -2e+02)
    (Transformation|SetActorTransform (Math|Transform|MakeTransform "-1310.000000,2090.000000,250.000000" "0.000000,-50.000000,0.000000" "1.000000,1.000000,1.000000"))))

(fn ConstructionScript
  (|CallParentFunction))