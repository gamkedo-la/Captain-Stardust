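; Fire_Delivery_BP is a timed delivery world event that completes when a Carryable_BP of the expected class overlaps its DeliveryPoint, destroying that item.
; BeginPlay creates a countdown widget, which Tick updates as it decrements the remaining time.
; On expiry it destroys WaterBucket actors, and from inside that loop reuses the success path's cleanup.
; That shared cleanup hides the world event and countdown widgets, then destroys the event actor.
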(event OnComponentBeginOverlap(DeliveryPoint)
  (params (OverlappedComponent :type Primitive%20Component%20Object%20Reference) (OtherActor :type Actor%20Object%20Reference) (OtherComp :type Primitive%20Component%20Object%20Reference) (OtherBodyIndex :type Integer) (bFromSweep :type Boolean) (SweepResult :type Hit%20Result%20Structure%20%28by%20ref%29))
  (bind _classtoverify (Variables|Default|GetClassToVerify))
  ;[1 1 1] This can be an issue as it takes any Carryable object, not a specific one
  (bind _ascarryable_bp (Utilities|Casting|CastToCarryable_BP OtherActor))
  (if (== (Utilities|GetClass _ascarryable_bp) _classtoverify)
    (Development|PrintString (Utilities|GetClassDisplayName _classtoverify))
    (Actor|DestroyActor OtherActor)
    (Development|PrintString "Deliverable Deliered")
    ;[1 1 1] Remove UI after event is over
    (bind _foundwidgets (Widget|GetAllWidgetsOfClass "/Game/Blueprints/Widgets/WorldEvent_Widget.WorldEvent_Widget_C" true))
    (for _array_element _foundwidgets
      (Widget|SetVisibility _array_element "Hidden")
      (Development|PrintString "Should be hidden"))
    (bind _foundwidgets_2 (Widget|GetAllWidgetsOfClass "/Game/Blueprints/CountdownTime_UI_BP.CountdownTime_UI_BP_C" true))
    (for _array_element_2 _foundwidgets_2
      (Widget|SetVisibility _array_element_2 "Hidden")
      (Development|PrintString "Should be hidden also"))
    (Actor|DestroyActor)))

(event Custom|Timed
  ;[1 1 1] Timer Countdown
  ;;[1 1 1] Set 3rd Person location
  (bind _returnvalue (Actor|GetActorOfClass "/Game/ThirdPerson/Blueprints/BP_ThirdPersonCharacter.BP_ThirdPersonCharacter_C"))
  (Variables|Default|SetstartingPositionOf3rdPersonCharacter (Transformation|GetActorTransform _returnvalue))
  (Variables|Default|SetTime_Remaining (- (Variables|Default|GetTime_Remaining) (Utilities|Time|GetWorldDeltaSeconds)))
  ;;[1 1 1] Fail State - if Time Remaining <= 0
  (if (not (>= (Variables|Default|GetTime_Remaining) 0.0))
    (Development|PrintString "Time expired, mission has failed")
    ;[1 1 1] Remove Water bucket once fire is out
    (bind _outactors (Actor|GetAllActorsOfClass "/Game/Blueprints/Missions/WorldEvents/WaterBucket.WaterBucket_C"))
    (for _array_element _outactors
      (Actor|DestroyActor _array_element)
      ;[1 1 1] Remove UI after event is over
      (bind _foundwidgets (Widget|GetAllWidgetsOfClass "/Game/Blueprints/Widgets/WorldEvent_Widget.WorldEvent_Widget_C" true))
      (for _array_element_2 _foundwidgets
        (Widget|SetVisibility _array_element_2 "Hidden")
        (Development|PrintString "Should be hidden"))
      (bind _foundwidgets_2 (Widget|GetAllWidgetsOfClass "/Game/Blueprints/CountdownTime_UI_BP.CountdownTime_UI_BP_C" true))
      (for _array_element_3 _foundwidgets_2
        (Widget|SetVisibility _array_element_3 "Hidden")
        (Development|PrintString "Should be hidden also"))
      (Actor|DestroyActor))))

(event EventBeginPlay
  (Variables|Default|SetTime_Remaining (Variables|Default|GetStarting_Time))
  (bind _returnvalue (UserInterface|CreateWidget "/Game/Blueprints/CountdownTime_UI_BP.CountdownTime_UI_BP_C"))
  (Variables|Default|SetText%20Block%20Changing%20Time (Variables|/Game/Blueprints/CountdownTime_UI_BP.CountdownTime_UI_BP_C|GetTextBlock_ChangingTime _returnvalue))
  (UserInterface|Viewport|AddtoViewport _returnvalue 0)
  (Variables|Default|SettimeHasStarted true))

(event EventTick
  (params (DeltaSeconds :type Float%20%28single-precision%29))
  ;[1 1 1] Update the timer every frame
  (if (Variables|Default|GettimeHasStarted)
    (CallFunction|Timed)
    (Rendering|Components|TextRender|SetText (Variables|Default|GetText%20Block%20Changing%20Time) (Utilities|Text|ToText(Float) (Variables|Default|GetTime_Remaining) "HalfToEven"))))

(fn ConstructionScript)

(fn Timer)