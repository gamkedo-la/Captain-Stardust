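; Carryable pizza for a timed delivery world event.
; The first pickup spawns a timed PizzaDelivery actor that verifies this pizza class, while every pickup flags it as carried and enables mesh physics.
; Tick runs a despawn countdown; if it expires before any pickup, every WorldEventTrigger has its request cancelled, repeating each frame without destroying the pizza here.
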(event Custom|PizzaCountdown
  (bind _pickedupfirsttime (Variables|Default|GetPickedUpFirstTime))
  (bind _returnvalue (== _pickedupfirsttime false))
  ;[1 1 1] Countdown Timer
  (bind _output_get (Variables|Default|SetTimeTilDespawnIfNotInteractedWith (- (Variables|Default|GetTimeTilDespawnIfNotInteractedWith) (Utilities|Time|GetWorldDeltaSeconds))))
  (if (and (<= _output_get 0.0) _returnvalue)
    (Development|PrintString (Utilities|String|ToString(Float) _output_get))
    (Development|PrintString (Utilities|String|ToString(Boolean) _returnvalue))
    (bind _outactors (Actor|GetAllActorsOfClass "/Game/Blueprints/Missions/WorldEvents/WorldEventTrigger.WorldEventTrigger_C"))
    (for _array_element _outactors
      (Default|CancelRequest _array_element))))

(event EventBeginPlay
  (|CallParentFunction) ; This node is disabled and will not be called.\nDrag off pins to build functionality.
)

(event Collision|EventActorBeginOverlap
  (params (OtherActor :type Actor%20Object%20Reference))
  (|CallParentFunction OtherActor) ; This node is disabled and will not be called.\nDrag off pins to build functionality.
)

(event EventTick
  (params (DeltaSeconds :type Float%20%28single-precision%29))
  (|CallParentFunction DeltaSeconds)
  (CallFunction|PizzaCountdown))

(event EventPickUp
  (bind _output_get (Variables|Default|SetIsBeingCarry true))
  (Physics|SetSimulatePhysics (Variables|Character|GetMesh) _output_get)
  (if (Variables|Default|GetPickedUpFirstTime)
    (Development|PrintString "already picked up")
    (else
      (Development|PrintString "Start Timer")
      (Variables|Default|SetPickedUpFirstTime true)
      (bind _returnvalue (Game|SpawnActorfromClass "/Game/Blueprints/Missions/WorldEvents/PizzaDelivery.PizzaDelivery_C" (Variables|Default|GetPizzaSpawnArray) "Undefined" "MultiplyWithRoot" 0 0))
      (Variables|/Game/Blueprints/Missions/WorldEvents/PizzaDelivery.PizzaDelivery_C|SetisTimed _returnvalue true)
      (Variables|/Game/Blueprints/Missions/WorldEvents/PizzaDelivery.PizzaDelivery_C|SetStarting_Time _returnvalue 3e+01)
      (Variables|/Game/Blueprints/Missions/WorldEvents/PizzaDelivery.PizzaDelivery_C|SetClassToVerify _returnvalue "Pizza_BP_C"))))

(fn ConstructionScript
  (|CallParentFunction))