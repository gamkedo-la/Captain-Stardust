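; SpaceObj_BP is a carryable world item that takes its look from a set of container meshes.
; On BeginPlay it picks a random mesh from ContainerMeshes and gives the actor a random rotation on all three axes.
; PickUp flags it as being carried, passes that true flag to SetSimulatePhysics, so physics turns on rather than off, and resets the rotation to zero.
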(event EventBeginPlay
  (bind _returnvalue (Math|Random|RandomFloatinRange 0.0 1.8e+02))
  (|CallParentFunction)
  (Components|StaticMesh|SetStaticMesh (Variables|Character|GetMesh) (.OutItem (Utilities|Array|Random (Variables|Default|GetContainerMeshes))))
  (Transformation|SetActorRotation (Math|Rotator|MakeRotator _returnvalue _returnvalue _returnvalue)))

(event Collision|EventActorBeginOverlap
  (params (OtherActor :type Actor%20Object%20Reference))
  (|CallParentFunction OtherActor) ; This node is disabled and will not be called.\nDrag off pins to build functionality.
)

(event EventPickUp
  (bind _output_get (Variables|Default|SetIsBeingCarry true))
  (Physics|SetSimulatePhysics (Variables|Character|GetMesh) _output_get)
  (Transformation|SetActorRotation (Math|Rotator|MakeRotator 0.0 0.0 0.0)))

(fn ConstructionScript
  (|CallParentFunction))