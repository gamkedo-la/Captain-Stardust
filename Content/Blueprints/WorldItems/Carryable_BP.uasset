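; Carryable world item that runs physics on its Mesh only while carried or moving.
; PickUp flags it as carried and enables simulation; Release clears the flag.
; Tick switches physics off for uncarried items once X velocity is near zero, ignoring Y and Z.
; A hit on a sleeping mesh re-enables physics, borrowing the carried flag for a 0.2-second grace period, with debug prints on toggles.
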(event OnComponentHit(Mesh)
  (params (HitComponent :type Primitive%20Component%20Object%20Reference) (OtherActor :type Actor%20Object%20Reference) (OtherComp :type Primitive%20Component%20Object%20Reference) (NormalImpulse :type Vector :default "0, 0, 0") (Hit :type Hit%20Result%20Structure%20%28by%20ref%29))
  (if (not (Physics|IsSimulatingPhysics (Variables|Default|GetMesh) "None"))
    (bind _output_get (Variables|Default|SetIsBeingCarry true))
    (Physics|SetSimulatePhysics (Variables|Default|GetMesh) _output_get)
    (Utilities|FlowControl|Delay 0.2)
    (Variables|Default|SetIsBeingCarry false)
    (Development|PrintString (Utilities|String|Append (Utilities|GetDisplayName self) ": PHY ON"))))

(event EventBeginPlay)

(event Collision|EventActorBeginOverlap
  (params (OtherActor :type Actor%20Object%20Reference)))

(event EventTick
  (params (DeltaSeconds :type Float%20%28single-precision%29))
  (bind _mesh (Variables|Default|GetMesh))
  (if (and (not (Variables|Default|GetIsBeingCarry)) (Physics|IsSimulatingPhysics _mesh "None"))
    (bind _returnvalue (Physics|GetPhysicsLinearVelocity _mesh "None"))
    (if (and (< (.x _returnvalue) 0.01) (> (.x _returnvalue) -0.01))
      (Physics|SetSimulatePhysics (Variables|Default|GetMesh) false)
      (Development|PrintString (Utilities|String|Append (Utilities|GetDisplayName self) ": PHY OFF")))))

(event EventRelease
  (Variables|Default|SetIsBeingCarry false))

(event EventPickUp
  (bind _output_get (Variables|Default|SetIsBeingCarry true))
  (Physics|SetSimulatePhysics (Variables|Default|GetMesh) _output_get)
  (Development|PrintString (Utilities|String|Append (Utilities|GetDisplayName self) ": PHY ON")))

(fn ConstructionScript)