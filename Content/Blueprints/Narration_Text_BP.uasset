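; Narration sequencer that shows timed character-name and dialogue lines in NarrativeText_Blueprint, creating the widget and starting on BeginPlay when AutoStart is set.
; StartDialog loops by index through parallel name, text and delay arrays, pushing each line to the widget.
; Past the end it hides the narration and, for InitialIntro, replaces objective widgets with the mission objective.
; KillItEarly forces the index high to cut the sequence short.
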(event Custom|StartDialog
  (bind _output_get (Variables|Default|SetIncrementSystem (+ (Variables|Default|GetIncrementSystem) 1) :!label _label))
  (bind _foundwidgets (Widget|GetAllWidgetsOfClass "/Game/Blueprints/Widgets/NarrativeText_Blueprint.NarrativeText_Blueprint_C" true))
  (bind _output_get_2 (Variables|Default|SetFound%20Widgets _foundwidgets))
  (Default|UpdateCharacterName _output_get_2 (Utilities|Array|Get(acopy) (Variables|Default|GetCharacterNameArray) _output_get))
  (Default|UpdateNarrationText _output_get_2 (Utilities|Array|Get(acopy) (Variables|Default|GetCharacterTextArray) _output_get))
  (Utilities|FlowControl|Delay (Utilities|Array|Get(acopy) (Variables|Default|GetTimeDelay) _output_get))
  (if (> (Variables|Default|GetIncrementSystem) (+ (Utilities|Array|Length (Variables|Default|GetCharacterNameArray)) 1))
    (bind _foundwidgets_2 (Widget|GetAllWidgetsOfClass "/Game/Blueprints/Widgets/NarrativeText_Blueprint.NarrativeText_Blueprint_C" true))
    (Widget|SetVisibility _foundwidgets_2 "Hidden")
    (if (Variables|Default|GetinitialIntro)
      (bind _foundwidgets_3 (Widget|GetAllWidgetsOfClass "/Game/Blueprints/Widgets/Objective_Widget.Objective_Widget_C" true))
      (for _array_element _foundwidgets_3
        (Widget|SetVisibility _array_element "Hidden"))
      (bind _returnvalue (UserInterface|CreateWidget "/Game/Blueprints/Widgets/Objective_Widget.Objective_Widget_C"))
      (UserInterface|Viewport|AddtoViewport _returnvalue 0)
      (Default|UpdateObjective _returnvalue (Variables|Default|GetMission%20Name))
      (Default|UpdateObjectiveText _returnvalue (Variables|Default|GetMission%20Description)))
    (else
      (goto _label))))

(event Custom|KillItEarly
  (Variables|Default|SetIncrementSystem 100))

(event EventBeginPlay
  (if (Variables|Default|GetautoStart)
    (bind _returnvalue (UserInterface|CreateWidget "/Game/Blueprints/Widgets/NarrativeText_Blueprint.NarrativeText_Blueprint_C"))
    (UserInterface|Viewport|AddtoViewport _returnvalue 0)
    (CallFunction|StartDialog)))

(fn ConstructionScript)