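; Captain Quasar enemy that homes on the player via ProjectileMovement and shoots at random short intervals.
; Tick picks behavior by distance: home and fire at mid range, halt and fire up close, halt when far; it also updates the health bar and a spawned waypoint.
; Energy, punch and vehicle overlaps deal damage; death drops health or stamina and notifies the player.
; Targeted/Untargeted events toggle a spiral marker.
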(event OnComponentBeginOverlap(Capsule)
  (params (OverlappedComponent :type Primitive%20Component%20Object%20Reference) (OtherActor :type Actor%20Object%20Reference) (OtherComp :type Primitive%20Component%20Object%20Reference) (OtherBodyIndex :type Integer) (bFromSweep :type Boolean) (SweepResult :type Hit%20Result%20Structure%20%28by%20ref%29))
  ;[1 1 1] Take Damage from Energy Attack
  (if (Actor|ActorHasTag OtherActor "Energy")
    (Variables|Default|SetdamageToDeal 5e+01)
    (CallFunction|FlyingEnergyDamage)
    (else
      ;[1 1 1] Hit With a Punch
      (if (Actor|ActorHasTag OtherActor "Punch")
        (bind _aspunch_bp (Utilities|Casting|CastToPunch_BP OtherActor))
        (Variables|Default|SetdamageToDeal (Variables|/Game/Blueprints/Punch_BP.Punch_BP_C|GetdamageToDeal _aspunch_bp))
        (CallFunction|FlyingEnergyDamage)
        (else
          ;[1 1 1] Hit With a Vehicle
          (if (Actor|ActorHasTag OtherActor "Vehicle")
            (Variables|Default|SetdamageToDeal 5e+01)
            (CallFunction|FlyingEnergyDamage)))))))

(event Custom|FlyingEnergyDamage
  (bind _returnvalue (Transformation|GetActorTransform))
  ;[1 1 1] Lose Health if hit by Energy
  (Variables|Default|SetEnemy_Health (- (Variables|Default|GetEnemy_Health) (Variables|Default|GetdamageToDeal)))
  (if (<= (Variables|Default|GetEnemy_Health) 0.0)
    ;[1 1 1] Spawn either Health or Stamina after death
    (if (> (Math|Random|RandomIntegerinRange 0 10) 5)
      (Game|SpawnActorfromClass "/Game/Blueprints/HealthPickUp_BP.HealthPickUp_BP_C" _returnvalue "Undefined" "MultiplyWithRoot" 0 0)
      (else
        (Game|SpawnActorfromClass "/Game/Blueprints/StaminaPickup_BP.StaminaPickup_BP_C" _returnvalue "Undefined" "MultiplyWithRoot" 0 0)))
    (bind _asbp_third_person_character (Utilities|Casting|CastToBP_ThirdPersonCharacter (Game|Player|GetPlayerPawn 0)))
    (Default|SentryKilled _asbp_third_person_character)
    (Actor|DestroyActor)))

(event EventBeginPlay
  ;[1 1 1] Set the homing target at player when spawned
  (Utilities|FlowControl|Sequence
    (:then_0
      (bind _asbp_third_person_character (Utilities|Casting|CastToBP_ThirdPersonCharacter (Game|Player|GetPlayerPawn 0)))
      (Variables|/Script/Engine.ProjectileMovementComponent|SetHomingTargetComponent (Variables|Default|GetProjectileMovement) (Variables|/Script/Engine.Character|GetCapsuleComponent _asbp_third_person_character)))
    (:then_1
      ;[1 1 1] Enemy indicator on Waypoint
      (bind _returnvalue (Game|SpawnActorfromClass "/Game/Blueprints/Minimap/BP_Waypoint.BP_Waypoint_C" (Transformation|GetWorldTransform (Variables|Character|GetMesh)) "Undefined" "MultiplyWithRoot" 0 0)))))

(event EventTargeted
  ;[1 1 1] Show the circle beneath if targeted
  (Development|SetHiddeninGame (Variables|Default|GetSpiral) false false))

(event EventTick
  (params (DeltaSeconds :type Float%20%28single-precision%29))
  (bind _projectilemovement (Variables|Default|GetProjectileMovement))
  (Utilities|FlowControl|Sequence
    (:then_0
      ;[1 1 1] Set up Health Bar above Head
      (bind _asenemy_health_ui_bp (Utilities|Casting|CastToEnemy_Health_UI_BP (UserInterface|GetWidget (Variables|Default|GetHealthBarWidget))))
      (Progress|SetPercent (Variables|/Game/Blueprints/Enemies/Enemy_Health_UI_BP.Enemy_Health_UI_BP_C|GetHealthBar _asenemy_health_ui_bp) (/ (Variables|Default|GetEnemy_Health) (Variables|Default|GetEnemy_Max_Health))))
    (:then_1
      ;[1 1 1] If the player is > X and < Y, shoot at the player
      (bind _returnvalue (Actor|GetActorOfClass "/Game/ThirdPerson/Blueprints/BP_ThirdPersonCharacter.BP_ThirdPersonCharacter_C"))
      (if (and (< (Math|Vector|VectorLength (- (.location (Transformation|GetActorTransform _returnvalue)) (.location (Transformation|GetActorTransform)))) 1.5e+03) (> (Math|Vector|VectorLength (- (.location (Transformation|GetActorTransform _returnvalue)) (.location (Transformation|GetActorTransform)))) 5e+02))
        (Variables|/Script/Engine.ProjectileMovementComponent|SetbIsHomingProjectile _projectilemovement true)
        ;[1 1 1] Fire Bullet every .25-1 seconds
        (Utilities|FlowControl|Delay (Math|Random|RandomFloatinRange 0.25 1.0) :!label _label)
        (Game|SpawnActorfromClass "/Game/Blueprints/Enemy_Bullet_BP.Enemy_Bullet_BP_C" (Transformation|GetWorldTransform (Variables|Default|GetSpawnPoint)) "Undefined" "MultiplyWithRoot" 0 0)
        (else
          ;[1 1 1] If <500, stop movement, but fire bullet
          (if (<= (Math|Vector|VectorLength (- (.location (Transformation|GetActorTransform _returnvalue)) (.location (Transformation|GetActorTransform)))) 5e+02)
            (Game|Components|ProjectileMovement|SetVelocityinLocalSpace _projectilemovement "0, 0, 0")
            (goto _label)
            (else
              ;[1 1 1] if >2000 stop movement, no firing
              (Game|Components|ProjectileMovement|SetVelocityinLocalSpace _projectilemovement "0, 0, 0"))))))
    (:then_2
      ;[1 1 1] Enemy indicator on Waypoint
      (Transformation|SetActorTransform (stale EventBeginPlay _returnvalue) (Transformation|GetWorldTransform (Variables|Character|GetMesh))))))

(event EventUntargeted
  ;[1 1 1] Show the circle beneath if targeted
  (Development|SetHiddeninGame (Variables|Default|GetSpiral) true false))

(fn ConstructionScript)