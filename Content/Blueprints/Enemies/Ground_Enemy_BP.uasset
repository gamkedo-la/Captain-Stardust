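; Ground enemy that roams the navmesh, fires Laser_BP projectiles and chases the player once spotted.
; RandomRoam loops moves and shots from random spawn points; PawnSensing triggers FollowPlayer, which fires after a random delay at mid range.
; Energy, punch and vehicle overlaps reduce health; death drops a health or stamina pickup.
; Tick updates the overhead health bar and its BP_Waypoint marker, while two custom events toggle a targeting spiral.
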(event OnSeePawn(PawnSensing)
  (params (Pawn :type Pawn%20Object%20Reference))
  ;[1 1 1] Enemy AI - Follow Player
  (Variables|Default|SetisSeeingPlayer true)
  (CallFunction|FollowPlayer))

(event OnComponentBeginOverlap(Trigger)
  (params (OverlappedComponent :type Primitive%20Component%20Object%20Reference) (OtherActor :type Actor%20Object%20Reference) (OtherComp :type Primitive%20Component%20Object%20Reference) (OtherBodyIndex :type Integer) (bFromSweep :type Boolean) (SweepResult :type Hit%20Result%20Structure%20%28by%20ref%29))
  ;[1 1 1] Take Damage from Energy Attack
  (if (Actor|ActorHasTag OtherActor "Energy")
    (Variables|Default|SetdamageToDeal 5e+01)
    (CallFunction|TakeDamagefromEnergy)
    (else
      ;[1 1 1] Hit by Punch
      (if (Actor|ActorHasTag OtherActor "Punch")
        (bind _aspunch_bp (Utilities|Casting|CastToPunch_BP OtherActor))
        (Variables|Default|SetdamageToDeal (Variables|/Game/Blueprints/Punch_BP.Punch_BP_C|GetdamageToDeal _aspunch_bp))
        (CallFunction|TakeDamagefromEnergy)
        (else
          ;[1 1 1] Hit by Car
          (if (Actor|ActorHasTag OtherActor "Vehicle")
            (Variables|Default|SetdamageToDeal 5e+01)
            (CallFunction|TakeDamagefromEnergy)))))))

(event Custom|FollowPlayer
  ;[1 1 1] Enemy AI - Follow Player
  (if (Variables|Default|GetisSeeingPlayer)
    (AI|AIMoveTo self "0, 0, 0" (Game|GetPlayerCharacter 0) 5.0 false
      (:then
        ;[1 1 1] Spawn laser to attack player
        (bind _returnvalue (Actor|GetActorOfClass "/Game/ThirdPerson/Blueprints/BP_ThirdPersonCharacter.BP_ThirdPersonCharacter_C"))
        (if (and (< (Math|Vector|VectorLength (- (.location (Transformation|GetActorTransform _returnvalue)) (.location (Transformation|GetActorTransform)))) 1.5e+03) (> (Math|Vector|VectorLength (- (.location (Transformation|GetActorTransform _returnvalue)) (.location (Transformation|GetActorTransform)))) 5e+02))
          (Utilities|FlowControl|Delay (Math|Random|RandomFloatinRange 2.5 5.0))
          (Game|SpawnActorfromClass "/Game/Blueprints/Laser_BP.Laser_BP_C" (Math|Transform|MakeTransform (.location (Transformation|GetWorldTransform (Variables|Default|GetSpawnPoint))) "-90.000000,0.000000,0.000000" "1.000000,1.000000,1.000000") "Undefined" "MultiplyWithRoot" 0 0))))
    (else
      (CallFunction|RandomRoam))))

(event Custom|TakeDamageFromEnergy
  (bind _returnvalue (Transformation|GetActorTransform))
  ;[1 1 1] Lose Health if hit by Energy
  (Variables|Default|SetEnemy_Health (- (Variables|Default|GetEnemy_Health) (Variables|Default|GetdamageToDeal)))
  (if (<= (Variables|Default|GetEnemy_Health) 0.0)
    ;[1 1 1] Spawn either Health or Stamina after death
    (if (> (Math|Random|RandomIntegerinRange 0 10) 5)
      (Game|SpawnActorfromClass "/Game/Blueprints/HealthPickUp_BP.HealthPickUp_BP_C" _returnvalue "Undefined" "MultiplyWithRoot" 0 0)
      (else
        (Game|SpawnActorfromClass "/Game/Blueprints/StaminaPickup_BP.StaminaPickup_BP_C" _returnvalue "Undefined" "MultiplyWithRoot" 0 0)))
    (Actor|DestroyActor (stale EventBeginPlay _returnvalue))
    (Actor|DestroyActor)))

(event Custom|RandomRoam
  (bind _returnvalue (Math|Random|RandomInteger 4))
  ;[1 1 1] Randomly Walk if it doesn't se the player
  (AI|AIMoveTo self (.RandomLocation (AI|Navigation|GetRandomReachablePointinRadius (Transformation|GetActorLocation) 4e+03 0 0)) 0 5.0 false
    (:then
      _)
    (:OnSuccess
      _))
  (Utilities|FlowControl|Delay 6.0)
  (switch int _returnvalue
    (:Default
      (Game|SpawnActorfromClass "/Game/Blueprints/Laser_BP.Laser_BP_C" (Math|Transform|MakeTransform (.location (Transformation|GetWorldTransform (Variables|Default|GetSpawnPoint1))) "90.000000,0.000000,0.000000" "1.000000,1.000000,1.000000") "Undefined" "MultiplyWithRoot" 0 0 :!label _label))
    (:0
      (Game|SpawnActorfromClass "/Game/Blueprints/Laser_BP.Laser_BP_C" (Math|Transform|MakeTransform (.location (Transformation|GetWorldTransform (Variables|Default|GetSpawnPoint))) "-90.000000,90.000000,0.000000" "1.000000,1.000000,1.000000") "Undefined" "MultiplyWithRoot" 0 0))
    (:1
      (goto _label))
    (:2
      (Game|SpawnActorfromClass "/Game/Blueprints/Laser_BP.Laser_BP_C" (Math|Transform|MakeTransform (.location (Transformation|GetWorldTransform (Variables|Default|GetSpawnPoint2))) "-90.000000,0.000000,0.000000" "1.000000,1.000000,1.000000") "Undefined" "MultiplyWithRoot" 0 0))
    (:3
      (Game|SpawnActorfromClass "/Game/Blueprints/Laser_BP.Laser_BP_C" (Math|Transform|MakeTransform (.location (Transformation|GetWorldTransform (Variables|Default|GetSpawnPoint3))) "-90.000000,-90.000000,0.000000" "1.000000,1.000000,1.000000") "Undefined" "MultiplyWithRoot" 0 0)))
  (Development|PrintString (Utilities|String|ToString(Integer) _returnvalue))
  (CallFunction|RandomRoam))

(event Custom|CustomEvent
  ;[1 1 1] Show the circle beneath if targeted
  (Development|SetHiddeninGame (Variables|Default|GetSpiral) false false))

(event Custom|CustomEvent_1
  ;[1 1 1] Show the circle beneath if targeted
  (Development|SetHiddeninGame (Variables|Default|GetSpiral) true false))

(event EventTick
  (params (DeltaSeconds :type Float%20%28single-precision%29))
  ;[1 1 1] Set up Health Bar above Head
  (Utilities|FlowControl|Sequence
    (:then_0
      (bind _asenemy_health_ui_bp (Utilities|Casting|CastToEnemy_Health_UI_BP (UserInterface|GetWidget (Variables|Default|GetHealthBarWidget))))
      (Progress|SetPercent (Variables|/Game/Blueprints/Enemies/Enemy_Health_UI_BP.Enemy_Health_UI_BP_C|GetHealthBar _asenemy_health_ui_bp) (/ (Variables|Default|GetEnemy_Health) (Variables|Default|GetEnemy_Max_Health))))
    (:then_1
      ;[1 1 1] Enemy indicator on Waypoint
      (Transformation|SetActorTransform (stale EventBeginPlay _returnvalue) (Transformation|GetWorldTransform (Variables|Character|GetMesh))))))

(event EventBeginPlay
  ;[1 1 1] Enemy indicator on Waypoint
  (Utilities|FlowControl|Sequence
    (:then_0
      (bind _returnvalue (Game|SpawnActorfromClass "/Game/Blueprints/Minimap/BP_Waypoint.BP_Waypoint_C" (Transformation|GetWorldTransform (Variables|Character|GetMesh)) "Undefined" "MultiplyWithRoot" 0 0)))
    (:then_1
      (CallFunction|RandomRoam))))

(fn ConstructionScript)